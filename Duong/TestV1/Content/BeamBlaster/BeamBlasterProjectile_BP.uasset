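; BeamBlasterProjectile_BP is the projectile for the Beam Blaster, damaging only its assigned target on contact.
; BeginPlay runs the parent logic, then sets damage and projectile speed; the file itself contains no movement code.
; When the Trigger component overlaps the actor stored in TargetRun, it applies damage, spawns an impact particle effect and destroys itself, ignoring all other actors.
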(event `self.ReceiveBeginPlay`
  (`parent.ReceiveBeginPlay`)
  (set `self.Damage` 10.0)
  (set `self.ProjectileSpeed` 45.0))

(event `self.Trigger.OnComponentBeginOverlap`
  (params (OverlappedComponent :type "PrimitiveComponent Object Reference") (OtherActor :type "Actor Object Reference") (OtherComp :type "PrimitiveComponent Object Reference") (OtherBodyIndex :type Integer) (bFromSweep :type Boolean) (SweepResult :type "HitResult Structure (by ref)"))
  (bind _targetrun (`self.TargetRun`))
  (`/Engine/EditorBlueprintResources/StandardMacros.IsValid` OtherActor
    (:`Is Valid`
      (if (== _targetrun OtherActor)
        (`GameplayStatics.ApplyDamage` _targetrun (`self.Damage`))
        (`GameplayStatics.SpawnEmitterAtLocation` "/Game/BeamBlaster/VFX/BeamBlasterMuzzleImpact.BeamBlasterMuzzleImpact" (`self.K2_GetActorLocation`))
        (`self.K2_DestroyActor`)))))

(fn `UserConstructionScript`
  (`parent.UserConstructionScript`))