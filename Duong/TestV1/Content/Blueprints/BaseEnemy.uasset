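; Base enemy character that provides shared health and movement speed functions.
; BeginPlay caches the CharacterMovement max walk speed as the default run speed.
; ModifyHealth subtracts damage from the current value in the Health struct and returns health and a death flag, without handling death itself.
; ChangeRunSpeed raises or lowers speed by a percentage of that cached default, so changes do not stack, and ResetRunSpeed restores it.
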(event `self.ReceiveBeginPlay`
  (set `self.DefaultRunSpeed` (`CharacterMovementComponent.MaxWalkSpeed` (`self.CharacterMovement`))))

(fn `ChangeRunSpeed`
  (params (Percent :type "Float (double-precision)") (Increase :type Boolean))
  (bind _charactermovement (`self.CharacterMovement`))
  (bind _returnvalue (* (/ Percent 100.0) (`self.DefaultRunSpeed`)))
  (if Increase
    (set `CharacterMovementComponent.MaxWalkSpeed` (+ _returnvalue (`self.DefaultRunSpeed`)) _charactermovement)
    (else
      (set `CharacterMovementComponent.MaxWalkSpeed` (- (`self.DefaultRunSpeed`) _returnvalue) _charactermovement))))

(fn `Modify Health`
  (params (Damage :type "Float (double-precision)"))
  (returns (Health :type "Float (double-precision)") (IsDeath :type Boolean))
  (bind (_health_max _health_current) (break `/Game/Blueprints/HealthStruct` (`self.Health`)))
  (bind _returnvalue (- _health_current Damage))
  (set `self.Health` (make `/Game/Blueprints/HealthStruct` _health_max _returnvalue))
  (return _returnvalue (<= _health_current 0.0)))

(fn `Reset Run Speed`
  (set `CharacterMovementComponent.MaxWalkSpeed` (`self.DefaultRunSpeed`) (`self.CharacterMovement`)))

(fn `UserConstructionScript`)