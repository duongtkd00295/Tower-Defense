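; BaseProjectile is a homing projectile actor that chases its TargetRun actor and destroys itself when that reference is no longer valid.
; Each Tick calls UpdateRotation, which sets rotation through RInterpTo toward the target's look-at rotation, then steps forward by ProjectileSpeed.
; The step is per frame, not scaled by delta time, and uses SetActorRelativeLocation without sweep.
; It contains no hit or damage logic.
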(event `self.ReceiveTick`
  (params (DeltaSeconds :type "Float (single-precision)"))
  (set `self.DeltaTime` DeltaSeconds)
  (`self.UpdateRotation`))

(event `UpdateRotation`
  (bind _returnvalue (`self.K2_GetActorRotation`))
  ;[1 1 1] Update Rotation And Location
  (`/Engine/EditorBlueprintResources/StandardMacros.IsValid` (`self.TargetRun`)
    (:`Is Valid`
      (`self.K2_SetActorRotation` (`KismetMathLibrary.RInterpTo` _returnvalue (`KismetMathLibrary.FindLookAtRotation` (`self.K2_GetActorLocation`) (`self.K2_GetActorLocation` (`self.TargetRun`))) (`self.DeltaTime`)))
      (`self.K2_SetActorRelativeLocation` (+ (* (`KismetMathLibrary.GetForwardVector` _returnvalue) (`self.ProjectileSpeed`)) (`self.K2_GetActorLocation`))))
    (:`Is Not Valid`
      (`self.K2_DestroyActor`))))

(fn `UserConstructionScript`)