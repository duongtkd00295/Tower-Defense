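; BaseTower is a base tower Blueprint that supplies target selection against BaseEnemy actors, with its event graph and construction script left empty.
; ClosestTarget takes an array of hit results, casts each hit actor to BaseEnemy, and returns the nearest one with health above zero.
; It tracks the best candidate and its distance from the tower in temporary variables while looping.
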(fn `ClosestTarget`
  (params (Hits :type "Array of HitResult Structure"))
  (returns (Target :type "/Game/Blueprints/BaseEnemy Object Reference"))
  (locals (TempTarget :type "/Game/Blueprints/BaseEnemy Object Reference") (TempDistance :type "Float (double-precision)" :default 0.0))
  (for _array_element Hits
    (bind (_bblockinghit _binitialoverlap _time _distance _location _impactpoint _normal _impactnormal _physmat _hitactor) (`GameplayStatics.BreakHitResult` _array_element))
    (bind _asbase_enemy (cast `/Game/Blueprints/BaseEnemy` _hitactor))
    (`/Engine/EditorBlueprintResources/StandardMacros.IsValid` (`local.TempTarget`)
      (:`Is Valid`
        (bind _returnvalue (`KismetMathLibrary.VSize` (- (`self.K2_GetActorLocation`) (`self.K2_GetActorLocation` _hitactor))))
        (if (and (< _returnvalue (`local.TempDistance`)) (> (`/Game/Blueprints/BaseEnemy.Health` _asbase_enemy) 0.0))
          (set `local.TempTarget` _asbase_enemy)
          (set `local.TempDistance` _returnvalue)))
      (:`Is Not Valid`
        (if (> (`/Game/Blueprints/BaseEnemy.Health` _asbase_enemy) 0.0)
          (set `local.TempTarget` _asbase_enemy)
          (set `local.TempDistance` _returnvalue)))))
  (return (`local.TempTarget`)))

(fn `UserConstructionScript`)