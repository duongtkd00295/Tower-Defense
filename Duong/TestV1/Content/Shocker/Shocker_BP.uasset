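; Shocker actor, apparently a defensive tower, that zaps one BaseEnemy at a time inside its trigger volume and reduces its run speed.
; Tick fires a beam from the EnergyBall socket with impact and stun particles, gated by a one-second cooldown.
; Overlap events set and clear the target, storing the old one.
; Without a target, a throttled search runs an insertion sort by distance from the old target, though it stops after the first overlapping enemy.
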(event `self.ReceiveBeginPlay`
  (`parent.ReceiveBeginPlay`))

(event `self.ReceiveTick`
  (params (DeltaSeconds :type "Float (single-precision)"))
  (`parent.ReceiveTick` DeltaSeconds)
  (`/Engine/EditorBlueprintResources/StandardMacros.IsValid` (`self.CurrentTarget`)
    (:`Is Valid`
      (if (not (`self.Shooting`))
        (`self.Create Zap`)))
    (:`Is Not Valid`
      (if (not (`self.CheckForTarget`))
        (`self.CheckNewTarget`)))))

(event `self.TriggerVolume.OnComponentBeginOverlap`
  (params (OverlappedComponent :type "PrimitiveComponent Object Reference") (OtherActor :type "Actor Object Reference") (OtherComp :type "PrimitiveComponent Object Reference") (OtherBodyIndex :type Integer) (bFromSweep :type Boolean) (SweepResult :type "HitResult Structure (by ref)"))
  (`/Engine/EditorBlueprintResources/StandardMacros.IsValid` OtherActor
    (:`Is Valid`
      (`/Engine/EditorBlueprintResources/StandardMacros.IsValid` (`self.CurrentTarget`)
        (:`Is Not Valid`
          (bind _asbase_enemy (cast `/Game/Blueprints/BaseEnemy` OtherActor))
          (set `self.CurrentTarget` _asbase_enemy))))))

(event `self.TriggerVolume.OnComponentEndOverlap`
  (params (OverlappedComponent :type "PrimitiveComponent Object Reference") (OtherActor :type "Actor Object Reference") (OtherComp :type "PrimitiveComponent Object Reference") (OtherBodyIndex :type Integer))
  (bind _currenttarget (`self.CurrentTarget`))
  (`/Engine/EditorBlueprintResources/StandardMacros.IsValid` OtherActor
    (:`Is Valid`
      (if (== OtherActor _currenttarget)
        (set `self.OldTarget` _currenttarget)
        (set `self.CurrentTarget` null)))))

(event `Create Zap`
  (bind _currenttarget (`self.CurrentTarget`))
  (bind _returnvalue (`self.K2_GetActorLocation` _currenttarget))
  (bind _returnvalue_2 (`SceneComponent.GetSocketLocation` (`self.EnergyBall`) (`KismetStringLibrary.Conv_StringToName` (`self.ShootSocketName`))))
  (set `self.Shooting` true)
  (bind _returnvalue_3 (`GameplayStatics.SpawnEmitterAtLocation` (`self.ParticleSystemZap`) _returnvalue_2))
  (bind _output_get (set `self.ParticleComponentZap` _returnvalue_3))
  (`ParticleSystemComponent.SetBeamSourcePoint` _output_get 0 _returnvalue_2 0)
  (`ParticleSystemComponent.SetBeamEndPoint` _output_get 0 _returnvalue)
  (`GameplayStatics.SpawnEmitterAtLocation` (`self.ParticleSystemZapImpact`) _returnvalue)
  (`GameplayStatics.SpawnEmitterAttached` (`self.ParticleSystemZapStun`) (`Character.Mesh` _currenttarget) "None" (0.0 0.0 0.0) (struct) (1.0 1.0 1.0) "SnapToTarget")
  (`/Game/Blueprints/BaseEnemy.ChangeRunSpeed` (`self.CurrentTarget`) 75.0 false)
  (`KismetSystemLibrary.Delay` 1.0)
  (set `self.Shooting` false))

(event `CheckNewTarget`
  (set `self.CheckForTarget` true)
  (bind _sortedlist (`self.Get Closest Target` (`PrimitiveComponent.GetOverlappingActors` (`self.TriggerVolume`) "/Game/Blueprints/BaseEnemy.BaseEnemy_C") (`self.OldTarget`) 1))
  (bind _output (`|GetArrayItem` _sortedlist))
  (`/Engine/EditorBlueprintResources/StandardMacros.IsValid` _output
    (:`Is Valid`
      (bind _asbase_enemy (cast `/Game/Blueprints/BaseEnemy` _output))
      (set `self.CurrentTarget` _asbase_enemy))
    (:`Is Not Valid`
      _))
  (`KismetSystemLibrary.Delay` 0.25)
  (set `self.CheckForTarget` false))

(fn `Get Closest Target`
  (params (List :type "Array of Actor Object Reference") (Target :type "Actor Object Reference") (Quantity :type Integer))
  (returns (SortedList :type "Array of Actor Object Reference"))
  (locals (TempTarget :type "Actor Object Reference") (CurrentTargetStepper :type Integer) (CurrentTargetDistance :type "Float (double-precision)") (SortingList :type "Array of Actor Object Reference") (TempQuantity :type Integer))
  (bind _currenttargetstepper (`local.CurrentTargetStepper`))
  (for (_array_element _array_index) List
    (set `local.TempTarget` _array_element)
    (set `local.CurrentTargetStepper` _array_index)
    (set `local.CurrentTargetDistance` (`self.GetHorizontalDistanceTo` Target (`local.TempTarget`)))
    (while (and (> (`self.GetHorizontalDistanceTo` Target (`|GetArrayItem` (`local.SortingList`) (- _currenttargetstepper 1))) (`local.CurrentTargetDistance`)) (> _currenttargetstepper 0))
      (`/Engine/EditorBlueprintResources/StandardMacros.DecrementInt` (`local.CurrentTargetStepper`)))
    (`KismetArrayLibrary.Array_Insert` (`local.SortingList`) (`local.TempTarget`) (`local.CurrentTargetStepper`))
    (`/Engine/EditorBlueprintResources/StandardMacros.IncrementInt` (`local.TempQuantity`)
      (:`  `
        (if (not (< (`local.TempQuantity`) Quantity))
          (break)))))
  (return (`local.SortingList`)))

(fn `ShootZap`)

(fn `UserConstructionScript`
  (`parent.UserConstructionScript`))