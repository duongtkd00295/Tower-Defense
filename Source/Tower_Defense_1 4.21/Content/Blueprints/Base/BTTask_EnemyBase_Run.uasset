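; Behavior tree task that runs a BaseEnemy along its PathNode array, toward a random point within each node.
; Each AI tick picks a new random point from the current node and issues AIMoveTo, incrementing IndexOfPaths whenever Move Finished fires.
; The task never finishes successfully; it ends as failed once the indexed node is invalid.
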(event `self.ReceiveTickAI`
  (params (OwnerController :type "AIController Object Reference") (ControlledPawn :type "Pawn Object Reference") (DeltaSeconds :type "Float (single-precision)"))
  (bind _asbase_enemy (cast `/Game/Blueprints/Base/BaseEnemy` ControlledPawn))
  (bind _output (`|GetArrayItem` (`/Game/Blueprints/Base/BaseEnemy.PathNode` _asbase_enemy) (`self.IndexOfPaths`)))
  (`/Engine/EditorBlueprintResources/StandardMacros.IsValid` _output
    (:`Is Valid`
      (bind _point (`/Game/Blueprints/PathNode.RandomPoint` _output))
      (`AITask_MoveTo.AIMoveTo` OwnerController _point null
        (:`OnMoveFinished`
          (`/Engine/EditorBlueprintResources/StandardMacros.IncrementInt` (`self.IndexOfPaths`)))))
    (:`Is Not Valid`
      (`self.FinishExecute` false))))