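; Base enemy character that awards Energy as level currency when killed through DestroyEnemy, and explodes without reward on hitting an actor tagged Server.
; ModifyHealth subtracts damage and returns a death flag, leaving destruction to the caller.
; Speed data initializes walk speed and animation rate; ChangeRunSpeed scales by percentage, adjusting animation only on decreases.
; ClearSlow sets a timer that restores both.
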(event `self.ReceiveBeginPlay`
  (`self.Initial`))

(event `ClearSlow`
  (params (Time :type "Float (double-precision)") (Loop :type Boolean))
  ;[1 1 1] ClearSlow
  (`KismetSystemLibrary.K2_SetTimerDelegate` (delegate `ResetSpeed`) Time Loop))

(event `ResetSpeed`
  ;[1 1 1] ClearSlow
  (`self.ResetRunSpeed`))

(event `DestroyEnemy`
  (bind _aslevel_state (cast `/Game/Blueprints/Base/LevelState` (`GameplayStatics.GetGameState`)))
  (bind _success (`/Game/Blueprints/Base/LevelState.ModifyCurrency` _aslevel_state (`self.Energy`) false))
  (if _success
    (`self.K2_DestroyActor`)))

(event `self.CapsuleComponent.OnComponentHit`
  (params (HitComponent :type "PrimitiveComponent Object Reference") (OtherActor :type "Actor Object Reference") (OtherComp :type "PrimitiveComponent Object Reference") (NormalImpulse :type "Vector Structure") (Hit :type "HitResult Structure (by ref)"))
  (if (`self.ActorHasTag` (`.HitActor` (`GameplayStatics.BreakHitResult` Hit)) (`KismetStringLibrary.Conv_StringToName` (`self.Server`)))
    (`GameplayStatics.SpawnEmitterAtLocation` "/Game/VFX/DeathExplosion/DeathExplosion.DeathExplosion" (`self.K2_GetActorLocation`))
    (`self.K2_DestroyActor`)))

(fn `ChangeRunSpeed`
  (params (Percent :type "Float (double-precision)") (Increase :type Boolean))
  (locals (NewLocalVar_0 :type "Float (double-precision)") (NewLocalVar_1 :type "Float (double-precision)" :default 0.0))
  (bind _returnvalue (/ Percent 100.0))
  (bind _speed_max (break `/Game/Blueprints/Base/Structs/SpeedStruct` (`self.Speed`)))
  (bind (_speed_max_2 _speed_rate) (break `/Game/Blueprints/Base/Structs/SpeedStruct` (`self.Speed`)))
  (set `local.NewLocalVar_0` (* _returnvalue _speed_max_2))
  (set `local.NewLocalVar_1` (* _returnvalue _speed_rate))
  (if Increase
    (set `CharacterMovementComponent.MaxWalkSpeed` (+ _speed_max (`local.NewLocalVar_0`)) (`self.CharacterMovement`))
    (else
      (set `CharacterMovementComponent.MaxWalkSpeed` (- _speed_max_2 (`local.NewLocalVar_0`)) (`self.CharacterMovement`))
      (set `self.AnimRate` (- _speed_rate (`local.NewLocalVar_1`))))))

(fn `Initial`
  (bind (_speed_max _speed_rate) (break `/Game/Blueprints/Base/Structs/SpeedStruct` (`self.Speed`)))
  (set `CharacterMovementComponent.MaxWalkSpeed` _speed_max (`self.CharacterMovement`))
  (set `self.AnimRate` _speed_rate))

(fn `ModifyHealth`
  (params (Damage :type "Float (double-precision)"))
  (returns (Health :type "Float (double-precision)") (IsDeath :type Boolean))
  (bind (_health_max _health_current) (break `/Game/Blueprints/Base/Structs/HealthStruct` (`self.Health`)))
  (bind _returnvalue (- _health_current Damage))
  (set `self.Health` (make `/Game/Blueprints/Base/Structs/HealthStruct` _health_max _returnvalue))
  (return _returnvalue (<= _health_current 0.0)))

(fn `ResetRunSpeed`
  (bind (_speed_max _speed_rate) (break `/Game/Blueprints/Base/Structs/SpeedStruct` (`self.Speed`)))
  (set `CharacterMovementComponent.MaxWalkSpeed` _speed_max (`self.CharacterMovement`))
  (set `self.AnimRate` _speed_rate))

(fn `UserConstructionScript`)