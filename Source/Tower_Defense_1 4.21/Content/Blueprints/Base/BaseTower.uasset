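; BaseTower is a tower base Blueprint that provides a helper for ordering a list of enemies by distance.
; SortEnemyListByDistance measures horizontal distance from a given target, falling back to the tower itself when that target is invalid.
; It builds the returned list by insertion sort, stepping back to each element's slot in ascending or descending order.
; The event graph and construction script hold no logic.
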(fn `SortEnemyListByDistance`
  (params (ListTarget :type "Array of Actor Object Reference") (Target :type "Actor Object Reference") (Descending :type Boolean))
  (returns (SortedList :type "Array of Actor Object Reference"))
  (locals (SortingList :type "Array of Actor Object Reference") (TempTarget :type "Actor Object Reference") (CurrentTargetStepper :type Integer :default 0) (TempQuantity :type Integer :default 0) (CurrentTargetDistance :type "Float (double-precision)" :default 0.0) (MainTarget :type "Actor Object Reference"))
  (bind _currenttargetdistance (`local.CurrentTargetDistance`))
  (bind _currenttargetstepper (`local.CurrentTargetStepper`))
  (bind _returnvalue (> _currenttargetstepper 0))
  (bind _returnvalue_2 (`self.GetHorizontalDistanceTo` (`local.MainTarget`) (`|GetArrayItem` (`local.SortingList`) (- _currenttargetstepper 1))))
  (`/Engine/EditorBlueprintResources/StandardMacros.IsValid` Target
    (:`Is Valid`
      (set `local.MainTarget` Target))
    (:`Is Not Valid`
      (set `local.MainTarget` self)))
  (for (_array_element _array_index) ListTarget
    (set `local.TempTarget` _array_element)
    (set `local.CurrentTargetStepper` _array_index)
    (set `local.CurrentTargetDistance` (`self.GetHorizontalDistanceTo` (`local.MainTarget`) (`local.TempTarget`)))
    (if Descending
      (while (and (< _returnvalue_2 _currenttargetdistance) _returnvalue)
        (`/Engine/EditorBlueprintResources/StandardMacros.DecrementInt` (`local.CurrentTargetStepper`) :!label _label))
      (else
        (while (and (> _returnvalue_2 _currenttargetdistance) _returnvalue)
          (goto _label))))
    (`KismetArrayLibrary.Array_Insert` (`local.SortingList`) (`local.TempTarget`) (`local.CurrentTargetStepper`)))
  (return (`local.SortingList`)))

(fn `UserConstructionScript`)