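; LevelState is a Blueprint that holds a level's Currency and Health values, with no active event logic.
; ModifyCurrency and ModifyHealth apply a change only if the result stays non-negative, negating the amount when Minus is set.
; ModifyHealth adds zero when Minus is false, so it can only change Health through the Minus path.
; Both return values repeat the check after the update, effectively testing the change a second time.
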(fn `ModifyCurrency`
  (params (Number :type "Float (double-precision)") (Minus :type Boolean))
  (returns (Success :type Boolean))
  (locals (TempNumber :type "Float (double-precision)"))
  (bind _returnvalue (+ (`self.Currency`) (`local.TempNumber`)))
  (bind _returnvalue_2 (>= _returnvalue 0.0))
  (if Minus
    (set `local.TempNumber` (* -1.0 Number))
    (else
      (set `local.TempNumber` Number)))
  (if _returnvalue_2
    (set `self.Currency` _returnvalue))
  (return _returnvalue_2))

(fn `ModifyHealth`
  (params (Number :type Integer) (Minus :type Boolean))
  (returns (Success :type Boolean))
  (locals (NewLocalVar_0 :type Integer))
  (bind _returnvalue (+ (`self.Health`) (`local.NewLocalVar_0`)))
  (bind _returnvalue_2 (>= _returnvalue 0))
  (if Minus
    (set `local.NewLocalVar_0` (* Number -1))
    (else
      (set `local.NewLocalVar_0` 0)))
  (if _returnvalue_2
    (set `self.Health` _returnvalue))
  (return _returnvalue_2))

(fn `UserConstructionScript`)