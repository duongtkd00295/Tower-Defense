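; Homing projectile for the Beam Blaster that chases a single target actor and damages it on contact.
; Each tick it rotates toward the target with RInterpTo and steps along its forward vector by a fixed speed, not scaled by delta time.
; It destroys itself if the target becomes invalid or changes from the one stored at BeginPlay.
; A trigger overlap with that target applies damage, spawns an impact emitter and destroys the projectile.
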(event `self.ReceiveBeginPlay`
  (set `self.OldTarget` (`self.TargetRun`)))

(event `self.ReceiveTick`
  (params (DeltaSeconds :type "Float (single-precision)"))
  (set `self.DeltaTime` DeltaSeconds)
  (`self.UpdateRotation`))

(event `self.Trigger.OnComponentBeginOverlap`
  (params (OverlappedComponent :type "PrimitiveComponent Object Reference") (OtherActor :type "Actor Object Reference") (OtherComp :type "PrimitiveComponent Object Reference") (OtherBodyIndex :type Integer) (bFromSweep :type Boolean) (SweepResult :type "HitResult Structure (by ref)"))
  (bind _targetrun (`self.TargetRun`))
  ;[1 1 1] Comment
  (`/Engine/EditorBlueprintResources/StandardMacros.IsValid` OtherActor
    (:`Is Valid`
      (if (== _targetrun OtherActor)
        (`GameplayStatics.ApplyDamage` _targetrun (`self.Damage`))
        (`GameplayStatics.SpawnEmitterAtLocation` (`self.MuzzleImpact`) (`self.K2_GetActorLocation`))
        (`self.K2_DestroyActor`)))))

(event `UpdateRotation`
  (bind _returnvalue (`self.K2_GetActorRotation`))
  (bind _targetrun (`self.TargetRun`))
  ;[1 1 1] Update Rotation And Location
  (`/Engine/EditorBlueprintResources/StandardMacros.IsValid` _targetrun
    (:`Is Valid`
      (if (!= _targetrun (`self.OldTarget`))
        (`self.K2_DestroyActor` :!label _label)
        (else
          (`self.K2_SetActorRotation` (`KismetMathLibrary.RInterpTo` _returnvalue (`KismetMathLibrary.FindLookAtRotation` (`self.K2_GetActorLocation`) (`self.K2_GetActorLocation` (`self.TargetRun`))) (`self.DeltaTime`)))
          (`self.K2_SetActorRelativeLocation` (+ (* (`KismetMathLibrary.GetForwardVector` _returnvalue) (`self.ProjectileSpeed`)) (`self.K2_GetActorLocation`))))))
    (:`Is Not Valid`
      (goto _label))))

(fn `UserConstructionScript`
  (`parent.UserConstructionScript`))