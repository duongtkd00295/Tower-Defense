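; Shocker tower that zaps and briefly slows enemies, with no damage applied in this graph.
; Tick retargets the enemy in its Trigger nearest FinishLoction and fires, gated by a one-second delay.
; Each shot beams from the energy ball to that target, then staggers arcs from the current target to Sphere-overlapping enemies, nearest first, capped by Quantity.
; SpawnZap handles beam, impact and stun particles plus the timed slow.
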(event `self.ReceiveTick`
  (params (DeltaSeconds :type "Float (single-precision)"))
  ;[1 1 1] Comment
  (if (> (`KismetArrayLibrary.Array_Length` (`PrimitiveComponent.GetOverlappingActors` (`self.Trigger`) "/Game/Blueprints/Base/BaseEnemy.BaseEnemy_C")) 0)
    (`self.CheckNewTarget`)
    (`/Engine/EditorBlueprintResources/StandardMacros.IsValid` (`self.CurrentTarget`)
      (:`Is Valid`
        (if (not (`self.Shooting`))
          (`self.Shoot`))))))

(event `self.Trigger.OnComponentEndOverlap`
  (params (OverlappedComponent :type "PrimitiveComponent Object Reference") (OtherActor :type "Actor Object Reference") (OtherComp :type "PrimitiveComponent Object Reference") (OtherBodyIndex :type Integer))
  (bind _currenttarget (`self.CurrentTarget`))
  ;[1 1 1] Khi quái ra khỏi trụ
  (`/Engine/EditorBlueprintResources/StandardMacros.IsValid` _currenttarget
    (:`Is Valid`
      (if (== OtherActor _currenttarget)
        (set `self.OldTarget` _currenttarget)
        (set `self.CurrentTarget` null)))))

(event `CheckNewTarget`
  ;[1 1 1] Check New Target
  (set `self.CheckForTarget` true)
  (bind _sortedlist (`self.SortEnemyListByDistance` (`PrimitiveComponent.GetOverlappingActors` (`self.Trigger`) "/Game/Blueprints/Base/BaseEnemy.BaseEnemy_C") (`self.FinishLoction`)))
  (bind _output (`|GetArrayItem` _sortedlist))
  (`/Engine/EditorBlueprintResources/StandardMacros.IsValid` _output
    (:`Is Valid`
      (bind _asbase_enemy (cast `/Game/Blueprints/Base/BaseEnemy` _output))
      (set `self.CurrentTarget` _asbase_enemy))
    (:`Is Not Valid`
      _))
  (set `self.CheckForTarget` false))

(event `Shoot`
  (bind _currenttarget (`self.CurrentTarget`))
  ;[1 1 1] Comment
  (set `self.Shooting` true)
  (bind _sortedlist (`self.SortEnemyListByDistance` (`PrimitiveComponent.GetOverlappingActors` (`self.Sphere`) "/Game/Blueprints/Base/BaseEnemy.BaseEnemy_C") _currenttarget))
  (`self.SpawnZap` (`self.K2_GetActorLocation` _currenttarget) (`SceneComponent.GetSocketLocation` (`self.EnegyBall`) "ShootPoint") _currenttarget)
  (`self.Shoot1` (`self.Quantity`) _sortedlist)
  (`KismetSystemLibrary.Delay` 1.0)
  (set `self.Shooting` false))

(event `Shoot1`
  (params (QuantityOfEnemy :type Integer) (Array :type "Array of Actor Object Reference"))
  ;[1 1 1] Comment
  (set `self.TempTarget1` (`self.CurrentTarget`))
  (bind (_arrayelement _array_index) (`/Game/Blueprints/Base/LoopMacro.EachLoopBreakWithDelay` Array 0.1 :!label _label)
    (:`LoopBody`
      (if (< _array_index QuantityOfEnemy)
        (`/Engine/EditorBlueprintResources/StandardMacros.IsValid` _arrayelement
          (:`Is Valid`
            (bind _asbase_enemy (cast `/Game/Blueprints/Base/BaseEnemy` _arrayelement))
            (`self.SpawnZap` (`self.K2_GetActorLocation` _asbase_enemy) (`self.K2_GetActorLocation` (`self.CurrentTarget`)) _asbase_enemy)
            (set `self.TempTarget1` _asbase_enemy)))
        (else
          (goto _label :!via `Break`))))))

(fn `SpawnZap`
  (params (TargetPoint :type "Vector Structure") (SourcePoint :type "Vector Structure") (Target :type "/Game/Blueprints/Base/BaseEnemy Object Reference"))
  (bind _returnvalue (`GameplayStatics.SpawnEmitterAtLocation` (`self.Zap`) SourcePoint))
  (`ParticleSystemComponent.SetBeamSourcePoint` _returnvalue 0 SourcePoint 0)
  (`ParticleSystemComponent.SetBeamEndPoint` _returnvalue 0 TargetPoint)
  (`GameplayStatics.SpawnEmitterAtLocation` (`self.ZapImpact`) TargetPoint)
  (`GameplayStatics.SpawnEmitterAttached` (`self.ZapStun`) (`Character.Mesh` Target) "None" (0.0 0.0 0.0) (struct) (1.0 1.0 1.0) "SnapToTarget")
  (`/Game/Blueprints/Base/BaseEnemy.ChangeRunSpeed` Target 75.0 false)
  (`/Game/Blueprints/Base/BaseEnemy.ClearSlow` Target 1.0 false))

(fn `UserConstructionScript`
  (`parent.UserConstructionScript`))