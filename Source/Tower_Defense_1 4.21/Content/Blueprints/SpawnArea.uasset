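; Spawn area actor that spawns AI enemies at random points inside its box, following waves read from a data table.
; Each wave nests turns, turn details and enemy quantities, with data-driven delays between steps.
; A Status state machine on Tick dispatches the Get events, which advance indices and set the next state after any delay.
; Clear flags can hold progression until CheckClear finds no BaseEnemy actors left in the world.
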(event `self.ReceiveBeginPlay`
  ;[1 1 1] Begin Play
  (`self.GetWave`))

(event `GetEnemy`
  (bind _box (`self.Box`))
  (bind (_enemy _nextenemy _isclear _quantity) (break `/Game/Blueprints/Base/TurnEnemyStruct` (`self.CurrentTurnDetails`)))
  ;[1 1 1] Get Enemy
  (set `self.Status` 0)
  (if (< (`self.TempIndex`) _quantity)
    (`AIBlueprintHelperLibrary.SpawnAIFromClass` _enemy null (`KismetMathLibrary.RandomPointInBoundingBox` (`SceneComponent.K2_GetComponentLocation` _box) (`BoxComponent.GetScaledBoxExtent` _box)))
    (`/Engine/EditorBlueprintResources/StandardMacros.IncrementInt` (`self.TempIndex`)
      (:`  `
        (`KismetSystemLibrary.Delay` _nextenemy)
        (set `self.Status` 4)))
    (else
      (`/Engine/EditorBlueprintResources/StandardMacros.IncrementInt` (`self.IndexOfTurnDetails`)
        (:`  `
          (set `self.TempIndex` 0)
          (set `self.IsEnemyClear` _isclear)
          (set `self.Status` 3))))))

(event `GetWave`
  ;[1 1 1] Get Wave
  (set `self.Status` 0)
  (bind _outrownames (`DataTableFunctionLibrary.GetDataTableRowNames` (`self.TableData`)))
  (bind _returnvalue (`|GetDataTableRow` (`self.TableData`) (`|GetArrayItem` _outrownames (`self.IndexOfWave`)))
    (:`then`
      (bind _output_get (set `self.CurrentWave` _returnvalue))
      (bind (_turn _isclear _timestart) (break `/Game/Blueprints/Base/WaveStruct` _output_get))
      (set `self.IsClearWave` _isclear)
      (`KismetSystemLibrary.Delay` _timestart)
      (set `self.Status` 2))
    (:`RowNotFound`
      (set `self.IsPlay` false))))

(event `GetTurn`
  (bind _indexofturn (`self.IndexOfTurn`))
  (bind (_turn _isclear _timestart _timenext) (break `/Game/Blueprints/Base/WaveStruct` (`self.CurrentWave`)))
  ;[1 1 1] Get Turn
  (set `self.Status` 0)
  (if (< _indexofturn (`KismetArrayLibrary.Array_Length` _turn))
    (set `self.CurrentTurn` (`|GetArrayItem` _turn _indexofturn))
    (set `self.IsClearTurn` _isclear)
    (set `self.Status` 3)
    (else
      (`/Engine/EditorBlueprintResources/StandardMacros.IncrementInt` (`self.IndexOfWave`)
        (:`  `
          (set `self.IndexOfTurn` 0)
          (`KismetSystemLibrary.Delay` _timenext)
          (set `self.Status` 1))))))

(event `GetTurnDetails`
  (bind _indexofturndetails (`self.IndexOfTurnDetails`))
  (bind (_turnenemy _timenext _timestart _isclear) (break `/Game/Blueprints/Base/TurnStruct` (`self.CurrentTurn`)))
  ;[1 1 1] Get Turn Details
  (set `self.Status` 0)
  (if (< _indexofturndetails (`KismetArrayLibrary.Array_Length` _turnenemy))
    (set `self.CurrentTurnDetails` (`|GetArrayItem` _turnenemy _indexofturndetails))
    (set `self.IsTurnDetailsClear` _isclear)
    (`KismetSystemLibrary.Delay` _timestart)
    (set `self.Status` 4)
    (else
      (`/Engine/EditorBlueprintResources/StandardMacros.IncrementInt` (`self.IndexOfTurn`)
        (:`  `
          (set `self.IndexOfTurnDetails` 0)
          (`KismetSystemLibrary.Delay` _timenext)
          (set `self.Status` 2))))))

(event `self.ReceiveTick`
  (params (DeltaSeconds :type "Float (single-precision)"))
  ;[1 1 1] Event Tick
  (set `self.DeltaTime` DeltaSeconds)
  (switch `int` (`self.Status`)
    (:`1`
      (if (`self.IsClearWave`)
        (bind _isclear (`self.CheckClear`))
        (set `self.IsClearWave` _isclear)
        (else
          (`self.GetWave`))))
    (:`2`
      (if (`self.IsClearTurn`)
        (bind _isclear_2 (`self.CheckClear`))
        (set `self.IsClearTurn` _isclear_2)
        (else
          (`self.GetTurn`))))
    (:`3`
      (if (`self.IsTurnDetailsClear`)
        (bind _isclear_3 (`self.CheckClear`))
        (set `self.IsTurnDetailsClear` _isclear_3)
        (else
          (`self.GetTurnDetails`))))
    (:`4`
      (if (`self.IsEnemyClear`)
        (bind _isclear_4 (`self.CheckClear`))
        (set `self.IsEnemyClear` _isclear_4)
        (else
          (`self.GetEnemy`))))))

(fn `CheckClear`
  (returns (IsClear :type Boolean))
  (bind _outactors (`GameplayStatics.GetAllActorsOfClass` "/Game/Blueprints/Base/BaseEnemy.BaseEnemy_C"))
  (return (> (`KismetArrayLibrary.Array_Length` _outactors) 0)))

(fn `UserConstructionScript`)