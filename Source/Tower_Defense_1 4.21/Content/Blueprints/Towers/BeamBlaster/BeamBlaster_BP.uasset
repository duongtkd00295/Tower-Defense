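; BeamBlaster tower that targets the enemy in its trigger volume closest to the finish location and fires projectiles at it.
; Each tick it re-sorts overlapping enemies to pick the target, then smoothly yaws the cannon toward it and sets IsShoot while it has health.
; Any end overlap on the volume clears the target.
; BaseShoot spawns a muzzle flash and a BeamBlaster projectile that receives the current target.
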(event `self.TriggerVolumer.OnComponentEndOverlap`
  (params (OverlappedComponent :type "PrimitiveComponent Object Reference") (OtherActor :type "Actor Object Reference") (OtherComp :type "PrimitiveComponent Object Reference") (OtherBodyIndex :type Integer))
  ;[1 1 1] Comment
  (set `self.OldTarget` null)
  (set `self.CurrentTarget` null))

(event `self.TriggerVolumer.OnComponentBeginOverlap`
  (params (OverlappedComponent :type "PrimitiveComponent Object Reference") (OtherActor :type "Actor Object Reference") (OtherComp :type "PrimitiveComponent Object Reference") (OtherBodyIndex :type Integer) (bFromSweep :type Boolean) (SweepResult :type "HitResult Structure (by ref)"))
  ;[1 1 1] On Overlap
)

(event `CheckNewTarget`
  ;[1 1 1] Check New Target
  (set `self.CheckForTarget` true)
  (bind _sortedlist (`self.SortEnemyListByDistance` (`PrimitiveComponent.GetOverlappingActors` (`self.TriggerVolumer`) "/Game/Blueprints/Base/BaseEnemy.BaseEnemy_C") (`self.FinishLoction`)))
  (bind _output (`|GetArrayItem` _sortedlist))
  (`/Engine/EditorBlueprintResources/StandardMacros.IsValid` _output
    (:`Is Valid`
      (bind _asbase_enemy (cast `/Game/Blueprints/Base/BaseEnemy` _output))
      (set `self.CurrentTarget` _asbase_enemy))
    (:`Is Not Valid`
      _))
  (`KismetSystemLibrary.Delay` 0.25)
  (set `self.CheckForTarget` false))

(event `UpdateRotation`
  (bind (_returnvalue_roll _returnvalue_pitch _returnvalue_yaw) (`KismetMathLibrary.BreakRotator` (`KismetMathLibrary.FindLookAtRotation` (`SceneComponent.K2_GetComponentLocation` (`self.Canon`)) (`self.K2_GetActorLocation` (`self.CurrentTarget`)))))
  ;[1 1 1] Update Rotation
  (`SceneComponent.K2_SetWorldRotation` (`self.Canon`) (`KismetMathLibrary.RInterpTo` (`SceneComponent.K2_GetComponentRotation` (`self.Canon`)) (`KismetMathLibrary.MakeRotator` 0.0 0.0 _returnvalue_yaw) (`self.DeltaTime`) 10.0) false false))

(event `self.ReceiveTick`
  (params (DeltaSeconds :type "Float (single-precision)"))
  (bind _currenttarget (`self.CurrentTarget`))
  (bind (_health_max _health_current) (break `/Game/Blueprints/Base/Structs/HealthStruct` (`/Game/Blueprints/Base/BaseEnemy.Health` _currenttarget)))
  ;[1 1 1] Event Tick
  (`parent.ReceiveTick` DeltaSeconds)
  (set `self.DeltaTime` DeltaSeconds)
  (`self.CheckNewTarget`)
  (`/Engine/EditorBlueprintResources/StandardMacros.IsValid` _currenttarget
    (:`Is Valid`
      (if (> _health_current 0.0)
        (`self.UpdateRotation`)
        (set `self.IsShoot` true)
        (else
          (set `self.IsShoot` false :!label _label))))
    (:`Is Not Valid`
      (goto _label))))

(fn `BaseShoot`
  (params (Point :type "SceneComponent Object Reference"))
  (locals (NewLocalVar_0 :type "Actor Class Reference"))
  (`GameplayStatics.SpawnEmitterAtLocation` (`self.MuzzleFlash`) (`SceneComponent.K2_GetComponentLocation` Point))
  (`|SpawnActorFromClass` "/Game/Blueprints/Towers/BeamBlaster/BeamBlaster_Projectile_BP.BeamBlaster_Projectile_BP_C" (`SceneComponent.K2_GetComponentToWorld` Point) "Undefined" "OverrideRootScale" null "/Game/Towers/BeamBlaster/VFX/BeamBlaster_Muzzle_Impact.BeamBlaster_Muzzle_Impact" (`self.CurrentTarget`) null))

(fn `UserConstructionScript`
  (`parent.UserConstructionScript`))